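; Moving platform actor that travels one way along an array of waypoint actors, with configurable mesh and material applied in the construction script.
; BeginPlay hides the waypoints and calls the start event from inside that loop, resetting to the first segment.
; MotionTimeline lerps the platform's relative location between waypoint world positions.
; Its event track advances the indices and replays the timeline until the last waypoint is the target.
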(event `self.ReceiveBeginPlay`
  ;[1 1 1] invisibility of the points o movent on platform 1
  (for _array_element (`self.waypoints`)
    (`self.SetActorHiddenInGame` _array_element true)
    (`self.platform start`)))

(event `platform start`
  (`self.setfirstwaypoint`)
  (`TimelineComponent.PlayFromStart` (`self.motion timeline`)))

(fn `path is finished`
  (returns (`is finished` :type Boolean))
  (return (== (`self.nextwaypointindex`) (- (`KismetArrayLibrary.Array_Length` (`self.waypoints`)) 1))))

(fn `set next waypoint`
  (bind _result (`/Engine/EditorBlueprintResources/StandardMacros.IncrementInt` (`self.currentwaypointindex`))
    (:`  `
      (set `self.nextwaypointindex` (+ _result 1))
      (`self.setpositions`))))

(fn `setfirstwaypoint`
  (set `self.currentwaypointindex` 0)
  (set `self.nextwaypointindex` 1)
  (`self.setpositions`))

(fn `setpositions`
  (bind _waypoints (`self.waypoints`))
  (set `self.currentwaypointposition` (`self.K2_GetActorLocation` (`|GetArrayItem` _waypoints (`self.currentwaypointindex`))))
  (set `self.nextwaypointposition` (`self.K2_GetActorLocation` (`|GetArrayItem` _waypoints (`self.nextwaypointindex`)))))

(fn `UserConstructionScript`
  (bind _platform_mesh (`self.Platform mesh`))
  (`StaticMeshComponent.SetStaticMesh` _platform_mesh (`self.Static_mesh`))
  (`PrimitiveComponent.SetMaterial` _platform_mesh 0 (`self.meterial`)))